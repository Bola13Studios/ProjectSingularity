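; BP_HealthStation is an interactable station that advertises an amount of HP for a price in hype.
; On BeginPlay it reads the Health row of DT_StationData and builds the StationInfo label from that amount and price.
; When its InteractiveStationComponent fires OnInteract, the station mesh briefly switches to an interaction material, then reverts after a delay.
; This graph handles only display and feedback, with no healing or payment logic.
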(event `self.ReceiveBeginPlay`
  (bind _returnvalue (`|GetDataTableRow` "/Game/Data/DataTables/DT_StationData.DT_StationData" "Health")
    (:`then`
      (bind _output_get (set `self.Out Row` _returnvalue))
      (bind (_m_type _m_typeamount _m_typeprice) (break `StationData` _output_get))
      (`TextRenderComponent.K2_SetText` (`self.StationInfo`) (`KismetTextLibrary.Conv_StringToText` (`KismetStringLibrary.Concat_StrStr` (`KismetStringLibrary.Concat_StrStr` (`KismetStringLibrary.Concat_StrStr` (`KismetStringLibrary.Concat_StrStr` (`KismetStringLibrary.Conv_DoubleToString` _m_typeamount) " HP") " \nfor \n") (`KismetStringLibrary.Conv_DoubleToString` _m_typeprice)) " hype"))))))

(event `self.InteractiveStationComponent.OnInteract`
  ; material change on health change
  (`PrimitiveComponent.SetMaterial` (`self.Station`) 0 "/Game/Graphics/Environment/Props/Stations/MI_StationInteraction.MI_StationInteraction")
  (`KismetSystemLibrary.Delay` 1.0)
  (`PrimitiveComponent.SetMaterial` (`self.Station`) 0 "/Game/Graphics/Environment/Props/Stations/MI_Station.MI_Station"))

(fn `UserConstructionScript`)