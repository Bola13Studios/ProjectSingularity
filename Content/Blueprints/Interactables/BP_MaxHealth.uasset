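; BP_MaxHealth is an interactable station, named for max health, that offers an amount of a stat mode in exchange for a Hype cost.
; On BeginPlay it builds the StationInfo label from the InteractiveStationComponent's amount, mode and cost.
; When the component fires OnInteract, the Station mesh briefly swaps to an interaction material, then reverts after a delay.
; The graph holds only this presentation logic and applies no stat change itself.
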(event `self.ReceiveBeginPlay`
  (`TextRenderComponent.K2_SetText` (`self.StationInfo`) (`KismetTextLibrary.Conv_StringToText` (`KismetStringLibrary.Concat_StrStr` (`KismetStringLibrary.Concat_StrStr` (`KismetStringLibrary.Concat_StrStr` (`KismetStringLibrary.Concat_StrStr` (`KismetStringLibrary.Conv_DoubleToString` (`InteractiveStation.amount` (`self.InteractiveStationComponent`))) (`|GetEnumeratorNameAsString` (`InteractiveStation.m_stationMode` (`self.InteractiveStationComponent`)))) " \nfor \n") (`KismetStringLibrary.Conv_DoubleToString` (`InteractiveStation.hypeCost` (`self.InteractiveStationComponent`)))) "Hype"))))

(event `self.InteractiveStationComponent.OnInteract`
  ; material change on health change
  (`PrimitiveComponent.SetMaterial` (`self.Station`) 0 "/Game/Graphics/Environment/Props/Stations/MI_StationInteraction.MI_StationInteraction")
  (`KismetSystemLibrary.Delay` 1.0)
  (`PrimitiveComponent.SetMaterial` (`self.Station`) 0 "/Game/Graphics/Environment/Props/Stations/MI_Station.MI_Station"))

(fn `UserConstructionScript`)