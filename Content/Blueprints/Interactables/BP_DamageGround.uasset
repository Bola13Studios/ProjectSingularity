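; BP_DamageGround is a hazard actor that damages BP_Player when it begins overlapping the actor.
; Each overlap applies one hit, passing the negated Damage value and itself as instigator to the player's Health component.
; A disconnected, never-run chain holds an older-style repeating damage loop for any Character with a BP_HealthComponent.
; The Box end-overlap still clears that loop's CharacterIsTouching flag, while its begin-overlap does nothing.
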(event `self.ReceiveActorBeginOverlap`
  (params (OtherActor :type "Actor Object Reference"))
  (bind _asbp_player (cast `/Game/Blueprints/Character/Player/BP_Player` OtherActor))
  (`HealthComponent.ChangeHealth` (`/Game/Blueprints/Character/Player/BP_Player.Health` _asbp_player) (* (`self.Damage`) -1.0) self))

(event `self.Box.OnComponentBeginOverlap`
  (params (OverlappedComponent :type "PrimitiveComponent Object Reference") (OtherActor :type "Actor Object Reference") (OtherComp :type "PrimitiveComponent Object Reference") (OtherBodyIndex :type Integer) (bFromSweep :type Boolean) (SweepResult :type "HitResult Structure (by ref)")))

(event `self.Box.OnComponentEndOverlap`
  (params (OverlappedComponent :type "PrimitiveComponent Object Reference") (OtherActor :type "Actor Object Reference") (OtherComp :type "PrimitiveComponent Object Reference") (OtherBodyIndex :type Integer))
  (cast `Character` OtherActor)
  (set `self.CharacterIsTouching` false))

(fn `UserConstructionScript`)