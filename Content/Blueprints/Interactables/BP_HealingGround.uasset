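; BP_HealingGround is an interactable area that heals characters standing inside its Box volume.
; On overlap it finds the character's BP_HealthComponent, adds a fixed amount of health and prints the current HP.
; A looped Delay repeats the heal every second until end overlap clears CharacterIsTouching.
; That flag and the stored character are single variables, so overlapping characters share one state.
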(event `self.Box.OnComponentBeginOverlap`
  (params (OverlappedComponent :type "PrimitiveComponent Object Reference") (OtherActor :type "Actor Object Reference") (OtherComp :type "PrimitiveComponent Object Reference") (OtherBodyIndex :type Integer) (bFromSweep :type Boolean) (SweepResult :type "HitResult Structure (by ref)"))
  (bind _ascharacter (cast `Character` OtherActor))
  (set `self.As Character` _ascharacter)
  (bind _returnvalue (`self.GetComponentByClass` _ascharacter "/Game/Blueprints/Components/BP_HealthComponent.BP_HealthComponent_C"))
  (if (`KismetSystemLibrary.IsValid` _returnvalue)
    (`HealthComponent.ChangeHealth` _returnvalue 15.0 null :!label _label)
    (set `self.CharacterIsTouching` true)
    (`KismetSystemLibrary.PrintString` (`KismetStringLibrary.Concat_StrStr` (`KismetSystemLibrary.GetDisplayName` (`self.As Character`)) " current HP is:  " (`KismetStringLibrary.Conv_DoubleToString` (`HealthComponent.GetHealth` _returnvalue))))
    (`KismetSystemLibrary.Delay` 1.0)
    (if (`self.CharacterIsTouching`)
      (goto _label))))

(event `self.Box.OnComponentEndOverlap`
  (params (OverlappedComponent :type "PrimitiveComponent Object Reference") (OtherActor :type "Actor Object Reference") (OtherComp :type "PrimitiveComponent Object Reference") (OtherBodyIndex :type Integer))
  (cast `Character` OtherActor)
  (set `self.CharacterIsTouching` false))

(fn `UserConstructionScript`)