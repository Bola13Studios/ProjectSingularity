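; BP_WeakPointZone is an environment actor that periodically moves a weak point to random spots within a box area.
; On BeginPlay it starts a looping timer that calls HandleSpawn at the spawn interval.
; HandleSpawn picks a random point inside the Area box's scaled extents, destroys the current weak point if valid, and spawns a new WeakPointClass actor there, keeping only one alive at a time.
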(event `self.ReceiveBeginPlay`
  (`KismetSystemLibrary.K2_SetTimer` null "HandleSpawn" (`self.SpawnInterval`) true))

(fn `GetRandomPointInArea`
  (returns (Output_Get :type "Vector Structure"))
  (locals (RandomPosition :type "Vector Structure"))
  (bind _area (`self.Area`))
  (bind (_returnvalue_x _returnvalue_y _returnvalue_z) (`KismetMathLibrary.BreakVector` (`BoxComponent.GetScaledBoxExtent` _area)))
  (bind (_returnvalue_x_2 _returnvalue_y_2 _returnvalue_z_2) (`KismetMathLibrary.BreakVector` (`SceneComponent.K2_GetComponentLocation` _area)))
  (bind _output_get (set `local.RandomPosition` (`KismetMathLibrary.MakeVector` (+ _returnvalue_x_2 (`KismetMathLibrary.RandomFloatInRange` (* _returnvalue_x -1.0) _returnvalue_x)) (+ _returnvalue_y_2 (`KismetMathLibrary.RandomFloatInRange` (* _returnvalue_y -1.0) _returnvalue_y)) (+ _returnvalue_z_2 (`KismetMathLibrary.RandomFloatInRange` (* _returnvalue_z -1.0) _returnvalue_z)))))
  (return _output_get))

(fn `HandleSpawn`
  (locals (TargetPosition :type "Vector Structure" :default (0.0 0.0 0.0)))
  (bind _output_get (`self.GetRandomPointInArea`))
  (set `local.TargetPosition` _output_get)
  (if (`KismetSystemLibrary.IsValid` (`self.CurrentWeakPoint`))
    (`self.K2_DestroyActor` (`self.CurrentWeakPoint`)))
  (bind _returnvalue (`|SpawnActorFromClass` (`self.WeakPointClass`) (`KismetMathLibrary.MakeTransform` (`local.TargetPosition`)) "Undefined" "MultiplyWithRoot" null null))
  (set `self.CurrentWeakPoint` _returnvalue))

(fn `UserConstructionScript`)