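; BP_Shop is a shop whose door and text sign open while the spawner manager is Waiting and close while it is On Going.
; Tick polls that state, holding off closing while the player overlaps AreaOfDetection by rechecking through a looping half-second Delay.
; OnOpen swaps the sign's text and color and plays the DoorOpen timeline, whose update sets the door straight to the target height without interpolation.
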(event `self.ReceiveBeginPlay`
  ; begin play
  ;; text
  (`TextRenderComponent.SetTextRenderColor` (`self.TextRender`) (`self.CloseColor`))
  (`TextRenderComponent.K2_SetText` (`self.TextRender`) (`self.CloseText`))
  ;; door
  (`PrimitiveComponent.SetMaterial` (`self.Door`) 0 (`self.CloseMaterial`))
  (`self.OnOpen` 0))

(event `self.ReceiveTick`
  (params (DeltaSeconds :type "Float (single-precision)"))
  (bind _spawnermanager (`self.SpawnerManager`))
  ; frame eater
  (if (`KismetSystemLibrary.IsValid` _spawnermanager)
    (switch `/Game/Blueprints/Enums/E_SpawnerState` (`/Game/Blueprints/Enemies/BP_SpawnManager.State` _spawnermanager)
      (:`NewEnumerator0`
        (`KismetSystemLibrary.PrintString` "on going" true false (struct :`G` 0.66 :`B` 1.0 :`A` 1.0) 2.0 "shop")
        (bind _asbp_player (cast `/Game/Blueprints/Character/Player/BP_Player` (`GameplayStatics.GetPlayerPawn` 0)))
        (if (== true (`PrimitiveComponent.IsOverlappingActor` (`self.AreaOfDetection`) _asbp_player)) :!label _label
          (`KismetSystemLibrary.Delay` 0.5)
          (goto _label)
          (else
            (`self.OnOpen` 0))))
      (:`NewEnumerator1`
        (`KismetSystemLibrary.PrintString` "waiting" true false (struct :`G` 0.66 :`B` 1.0 :`A` 1.0) 2.0 "shop")
        (`self.OnOpen` -700)))))

(event `OnOpen`
  (params (LastIndex :type Integer))
  (bind _textrender (`self.TextRender`))
  (bind _textrender_2 (`self.TextRender`))
  ; round trigger
  (if (!= LastIndex -700)
    (`TextRenderComponent.K2_SetText` _textrender_2 (`self.CloseText`))
    (`TextRenderComponent.SetTextRenderColor` _textrender_2 (`self.CloseColor`))
    (`Timeline|DoorOpen` :!label _label_2
      (:`Update`
        (`SceneComponent.K2_SetRelativeLocation` (`self.Door`) (`KismetMathLibrary.MakeVector` 0.0 0.0 (`KismetMathLibrary.Conv_IntToDouble` LastIndex)) false false)))
    (else
      (`TextRenderComponent.K2_SetText` _textrender (`self.OpenText`))
      (`TextRenderComponent.SetTextRenderColor` _textrender (`self.OpenColor`))
      (goto _label_2))))

(fn `UserConstructionScript`)