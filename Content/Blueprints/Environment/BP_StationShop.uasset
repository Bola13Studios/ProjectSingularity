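; BP_StationShop is a station shop that opens while the spawner manager is Waiting and closes during On Going rounds.
; Tick polls the manager state, delaying closure with a retry loop while the player overlaps the detection area.
; OnOpen updates the sign's text and color, then plays a timeline that sets both doors' Z directly to the target height, without interpolation.
; BeginPlay starts it closed.
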(event `self.ReceiveBeginPlay`
  ; begin play
  ;; text
  (`TextRenderComponent.SetTextRenderColor` (`self.Sign`) (`self.CloseCol`))
  (`TextRenderComponent.K2_SetText` (`self.Sign`) (`self.CloseTxt`))
  ;; door
  (`PrimitiveComponent.SetMaterial` (`self.DoorEntrance`) 0 (`self.CloseMat`))
  (`PrimitiveComponent.SetMaterial` (`self.DoorExit`) 0 (`self.CloseMat`))
  (`self.OnOpen` 0))

(event `self.ReceiveTick`
  (params (DeltaSeconds :type "Float (single-precision)"))
  (bind _spawnermanager (`self.SpawnerManager`))
  ; frame eater
  (if (`KismetSystemLibrary.IsValid` _spawnermanager)
    (switch `/Game/Blueprints/Enums/E_SpawnerState` (`/Game/Blueprints/Enemies/BP_SpawnManager.State` _spawnermanager)
      (:`NewEnumerator0`
        (`KismetSystemLibrary.PrintString` "on going" true false (struct :`G` 0.66 :`B` 1.0 :`A` 1.0) 2.0 "shop")
        (bind _asbp_player (cast `/Game/Blueprints/Character/Player/BP_Player` (`GameplayStatics.GetPlayerPawn` 0)))
        (if (== true (`PrimitiveComponent.IsOverlappingActor` (`self.AreaOfDetection`) _asbp_player)) :!label _label
          (`KismetSystemLibrary.Delay` 0.5)
          (goto _label)
          (else
            (`self.OnOpen` 0))))
      (:`NewEnumerator1`
        (`KismetSystemLibrary.PrintString` "waiting" true false (struct :`G` 0.66 :`B` 1.0 :`A` 1.0) 2.0 "shop")
        (`self.OnOpen` -700)))))

(event `OnOpen`
  (params (LastIndex :type Integer))
  (bind _returnvalue (`KismetMathLibrary.Conv_IntToDouble` LastIndex))
  (bind _sign (`self.Sign`))
  (bind _sign_2 (`self.Sign`))
  (bind _doorentrance (`self.DoorEntrance`))
  (bind _doorexit (`self.DoorExit`))
  (bind (_relativelocation_x _relativelocation_y) (`KismetMathLibrary.BreakVector` (`SceneComponent.RelativeLocation` _doorentrance)))
  (bind (_relativelocation_x_2 _relativelocation_y_2) (`KismetMathLibrary.BreakVector` (`SceneComponent.RelativeLocation` _doorexit)))
  ; round trigger
  (if (!= LastIndex -700)
    (`TextRenderComponent.K2_SetText` _sign_2 (`self.CloseTxt`))
    (`TextRenderComponent.SetTextRenderColor` _sign_2 (`self.CloseCol`))
    (`Timeline|OpenDoor` :!label _label_2
      (:`Update`
        (`SceneComponent.K2_SetRelativeLocation` _doorentrance (`KismetMathLibrary.MakeVector` _relativelocation_x _relativelocation_y _returnvalue) false false)
        (`SceneComponent.K2_SetRelativeLocation` _doorexit (`KismetMathLibrary.MakeVector` _relativelocation_x_2 _relativelocation_y_2 _returnvalue) false false)))
    (else
      (`TextRenderComponent.K2_SetText` _sign (`self.OpenTxt`))
      (`TextRenderComponent.SetTextRenderColor` _sign (`self.OpenCol`))
      (goto _label_2))))

(fn `UserConstructionScript`)