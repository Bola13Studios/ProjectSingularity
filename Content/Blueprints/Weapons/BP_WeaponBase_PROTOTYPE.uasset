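; Prototype base weapon Blueprint for a hitscan gun, currently using MP5 fire and idle animations.
; Tick advances a fire-rate timer and rebuilds the ray from the player 0 camera along its forward vector to MaxDistance.
; Shoot, gated by CanShoot and that timer, plays the fire animation and line-traces on Visibility, only drawing debug spheres at the impact or ray end, without damage.
; StopShoot restores the looping idle.
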(event `self.ReceiveBeginPlay`
  (set `self.CameraTransform` (`PlayerCameraManager.TransformComponent` (`PlayerController.PlayerCameraManager` (`GameplayStatics.GetPlayerController` 0)))))

(event `self.ReceiveTick`
  (params (DeltaSeconds :type "Float (single-precision)"))
  (bind _cameratransform (`self.CameraTransform`))
  (bind _returnvalue (`SceneComponent.K2_GetComponentLocation` _cameratransform))
  (set `self.FireRateElapsedTime` (+ DeltaSeconds (`self.FireRateElapsedTime`)))
  (set `self.RayCastStartPositon` _returnvalue)
  (set `self.RayCastEndPosition` (+ _returnvalue (* (`SceneComponent.GetForwardVector` _cameratransform) (`self.MaxDistance`)))))

(fn `Shoot`
  (if (and (`self.CanShoot`) (< (`self.FireRateTime`) (`self.FireRateElapsedTime`)))
    (set `self.FireRateElapsedTime` 0.0)
    (`SkeletalMeshComponent.PlayAnimation` (`self.SkeletalMesh`) "/Game/Graphics/Weapons/MP5/Animations/AS_Fire_MP5_W.AS_Fire_MP5_W" false)
    (bind (_outhit _returnvalue) (`KismetSystemLibrary.LineTraceSingle` (`self.RayCastStartPositon`) (`self.RayCastEndPosition`) "TraceTypeQuery1"))
    (if _returnvalue
      (`KismetSystemLibrary.DrawDebugSphere` (`.ImpactPoint` (`GameplayStatics.BreakHitResult` _outhit)) 5.0 12 (struct :`G` 1.0 :`B` 0.038204 :`A` 1.0) 1.0 1.0)
      (else
        (`KismetSystemLibrary.DrawDebugSphere` (`self.RayCastEndPosition`) 5.0 12 (struct :`G` 0.134315 :`B` 1.0 :`A` 1.0) 1.0 1.0)))
    (return)
    (else
      (return))))

(fn `StopShoot`
  (`SkeletalMeshComponent.PlayAnimation` (`self.SkeletalMesh`) "/Game/Graphics/Weapons/MP5/Animations/AS_Idle_MP5_W1.AS_Idle_MP5_W1" true)
  (return))

(fn `UserConstructionScript`)