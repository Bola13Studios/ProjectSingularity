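; BP_Hype is a trigger actor that awards hype points to a BP_TestFP each time one overlaps it.
; BeginPlay passes base points to its BPHypeComponent and, for a positive multiplier, also sets the multiplier, box color, tinted dynamic floor material and text labels for total and description.
; On overlap it adds the component's GetHype value to that actor and prints the award on screen.
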(event `self.ReceiveBeginPlay`
  (bind _multiplier (`self.Multiplier`))
  (bind _bp_hypecomponent (`self.BP_HypeComponent`))
  (set `/Game/Blueprints/Components/BP_HypeComponent.BaseValue` (`self.Points`) _bp_hypecomponent)
  (if (> _multiplier 0.0)
    (set `/Game/Blueprints/Components/BP_HypeComponent.Multiplier` _multiplier _bp_hypecomponent)
    (set `ShapeComponent.ShapeColor` (`self.BoxColor`) (`self.Box`))
    (bind _returnvalue (`PrimitiveComponent.CreateDynamicMaterialInstance` (`self.floor`) 0 null "None"))
    (`MaterialInstanceDynamic.SetVectorParameterValue` _returnvalue "Base Color" (`KismetMathLibrary.Conv_ColorToLinearColor` (`self.BoxColor`)))
    (`TextRenderComponent.K2_SetText` (`self.hype points`) (`KismetTextLibrary.Conv_DoubleToText` (* (`self.Points`) (`self.Multiplier`)) "HalfToEven"))
    (`TextRenderComponent.K2_SetText` (`self.description`) (`self.BoxDescription`))))

(event `self.ReceiveActorBeginOverlap`
  (params (OtherActor :type "Actor Object Reference"))
  (bind _finalvalue (`/Game/Blueprints/Components/BP_HypeComponent.GetHype` (`self.BP_HypeComponent`)))
  (bind _asbp_test_fp (cast `/Game/Blueprints/Character/BP_TestFP` OtherActor))
  (`/Game/Blueprints/Character/BP_TestFP.AddPoints` _asbp_test_fp _finalvalue)
  (`KismetSystemLibrary.PrintString` (`KismetStringLibrary.Concat_StrStr` (`KismetStringLibrary.Concat_StrStr` "Got " (`KismetStringLibrary.Conv_DoubleToString` _finalvalue)) " hype points!") true false (struct :`R` 1.0 :`G` 0.576629 :`B` 0.021212 :`A` 1.0) 2.0 "hype"))

(fn `UserConstructionScript`)