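; BP_SingleEnemySpawner is an enemy spawner that creates a configured enemy class and count for each round at its own transform.
; SpawnCurrentRoundEnemies indexes both arrays by round and loops through an execution wire and counter, spawning all in one call.
; Each enemy receives the SpawnManager reference, and the manager's enemy count increases.
; The logic that looks up BP_SpawnManager is disconnected, so this graph never assigns that reference.
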(event `self.ReceiveBeginPlay`)

(event `SpawnCurrentRoundEnemies`
  (params (CurrentRound :type Integer))
  (bind _output (`|GetArrayItem` (`self.EnemyToSpawn`) CurrentRound))
  (set `self.CurrentEnemy` _output)
  (if (`KismetSystemLibrary.IsValidClass` _output)
    (if (== (`|GetArrayItem` (`self.AmountToSpawn`) CurrentRound) (`self.Aux`)) :!label _label
      (set `self.Aux` 0)
      (else
        (bind _returnvalue (`|SpawnActorFromClass` (`self.CurrentEnemy`) (`self.GetTransform`) "Undefined" "MultiplyWithRoot" null null))
        (set `/Game/Blueprints/Enemies/BP_ChaserEnemy.SpawnManager` (`self.Spawn Manager`) _returnvalue)
        (`/Game/Blueprints/Enemies/BP_SpawnManager.IncreaseEnemyAmount` (`self.Spawn Manager`))
        (bind _result (`/Engine/EditorBlueprintResources/StandardMacros.IncrementInt` (`self.Aux`))
          (:`  `
            (set `self.Aux` _result)
            (goto _label)))))))

(fn `UserConstructionScript`)