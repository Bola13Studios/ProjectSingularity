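; Chaser enemy Blueprint that adds hit and attack color feedback plus a dash toward the player.
; Health changes trigger a red flash, while AttackFeedback drives a yellow one, both using timelines that lerp the mesh materials' Color parameter and stop after a delay.
; DashEnemy launches the character toward player 0 with velocity overridden, scaled by the dash force from its ChaserEnemyDataAsset.
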(event `self.ReceiveBeginPlay`
  (add `HealthComponent.OnHealthChanged` (`self.m_healthComponent`) (delegate `DamageFeedback`)))

(event `DamageFeedback`
  (params (Current :type "Float (single-precision)") (Max :type "Float (single-precision)") (Delta :type "Float (single-precision)") (InstigatorActor :type "Actor Object Reference"))
  (bind (_direction _newtrack_0) (`Timeline|Timeline_0` :!via `PlayFromStart` :!label _label)
    (:`Update`
      (`MeshComponent.SetColorParameterValueOnMaterials` (`self.Mesh`) "Color" (`KismetMathLibrary.LinearColorLerp` (struct :`R` 1.0 :`G` 1.0 :`B` 1.0) (struct :`R` 1.0 :`A` 1.0) _newtrack_0))
      (`KismetSystemLibrary.Delay` 1.0)
      (goto _label :!via `Stop`))))

(event `AttackFeedback`
  (bind (_direction _newtrack_0) (`Timeline|Timeline` :!via `PlayFromStart` :!label _label_2)
    (:`Update`
      (`MeshComponent.SetColorParameterValueOnMaterials` (`self.Mesh`) "Color" (`KismetMathLibrary.LinearColorLerp` (struct :`R` 1.0 :`G` 1.0 :`B` 1.0) (struct :`R` 1.0 :`G` 0.782079 :`A` 1.0) _newtrack_0))
      (`KismetSystemLibrary.Delay` 2.0)
      (goto _label_2 :!via `Stop`))))

(event `DashEnemy`
  (bind _aschaser_enemy_data_asset (cast `ChaserEnemyDataAsset` (`self.m_pCharacterDataAsset`)))
  (`self.LaunchCharacter` (* (`KismetMathLibrary.Normal` (- (`self.K2_GetActorLocation` (`GameplayStatics.GetPlayerPawn` 0)) (`self.K2_GetActorLocation`))) (`ChaserEnemyDataAsset.m_dashForce` _aschaser_enemy_data_asset)) true true))

(fn `UserConstructionScript`)