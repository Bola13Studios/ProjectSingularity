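; BP_SpawnManager runs round-based enemy spawning across the level's BP_SingleEnemySpawner actors.
; On BeginPlay it gathers those spawners and starts the first round.
; Each round it passes itself and the round index to every spawner, then increments the index.
; Increase and decrease events maintain a live enemy count, and the next round starts when a decrease brings it to zero.
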(event `DecreaseEnemyAmount`
  (bind _result (`/Engine/EditorBlueprintResources/StandardMacros.DecrementInt` (`self.EnemyAmount`))
    (:`  `
      (if (== _result 0)
        (`self.NextRound`)))))

(event `IncreaseEnemyAmount`
  (`/Engine/EditorBlueprintResources/StandardMacros.IncrementInt` (`self.EnemyAmount`)))

(event `self.ReceiveBeginPlay`
  (bind _outactors (`GameplayStatics.GetAllActorsOfClass` "/Game/Blueprints/Enemies/BP_SingleEnemySpawner.BP_SingleEnemySpawner_C"))
  (set `self.SpawnerList` _outactors)
  (`self.NextRound`))

(event `NextRound`
  (bind _current_round (`self.Current Round`))
  (for _array_element (`self.SpawnerList`)
    (set `/Game/Blueprints/Enemies/BP_SingleEnemySpawner.Spawn Manager` self _array_element)
    (`/Game/Blueprints/Enemies/BP_SingleEnemySpawner.SpawnCurrentRoundEnemies` _array_element _current_round))
  (`/Engine/EditorBlueprintResources/StandardMacros.IncrementInt` _current_round))

(fn `UserConstructionScript`)