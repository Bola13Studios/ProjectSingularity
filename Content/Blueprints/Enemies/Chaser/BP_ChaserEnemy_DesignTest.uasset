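; Design-test chaser enemy Blueprint that displays damage feedback and prints its health every tick.
; Health changes within a hit window are summed, with a restarted timer sending the total to a damage-number widget at one of four randomly cycled indices.
; Timelines tint the mesh red on damage and yellow for attack feedback.
; Dash and overlap-attack logic is disconnected, leaving those events empty and attack feedback untriggered here.
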(event `self.m_healthComponent.OnHealthChanged`
  (params (Current :type "Float (single-precision)") (Max :type "Float (single-precision)") (Delta :type "Float (single-precision)") (InstigatorActor :type "Actor Object Reference"))
  (if (!= Delta 0.0)
    (if (<= (- (`KismetSystemLibrary.GetGameTimeInSeconds`) (`self.LastHitTime`)) (`self.SumHitWindow`))
      (set `self.SumDamage` (+ Delta (`self.SumDamage`)))
      (set `self.LastHitTime` (`KismetSystemLibrary.GetGameTimeInSeconds`))
      (`KismetSystemLibrary.K2_ClearAndInvalidateTimerHandle` (`self.DamageTimerHandle`) :!label _label)
      (bind _returnvalue (`KismetSystemLibrary.K2_SetTimerDelegate` (delegate `ShowDamageWidget`) (`self.SumHitWindow`)))
      (set `self.DamageTimerHandle` _returnvalue)
      (else
        (set `self.SumDamage` Delta)
        (set `self.LastHitTime` (`KismetSystemLibrary.GetGameTimeInSeconds`))
        (if (`KismetSystemLibrary.K2_IsTimerActiveHandle` (`self.DamageTimerHandle`))
          (set `self.CurrentIndex` (`KismetMathLibrary.RandomIntegerInRange` 0 3) :!label _label_2)
          (if (== (`KismetArrayLibrary.Array_Find` (`self.UsedIndexesDamage`) (`self.CurrentIndex`)) -1)
            (`KismetArrayLibrary.Array_AddUnique` (`self.UsedIndexesDamage`) (`self.CurrentIndex`))
            (elif (>= (`KismetArrayLibrary.Array_Length` (`self.UsedIndexesDamage`)) 4)
              (`KismetArrayLibrary.Array_Clear` (`self.UsedIndexesDamage`))
              (else
                (goto _label_2))))
          (message `/Game/Blueprints/UI/DamageNumbers/BPI_DamNumWidget.DNW_Holder` (`WidgetComponent.GetUserWidgetObject` (`self.DamageNumbers`)) (`self.SumDamage`) (`self.CurrentIndex`))
          (else
            (goto _label)))))))

(event `ShowDamageWidget`
  (goto _label_2))

(event `self.ReceiveTick`
  (params (DeltaSeconds :type "Float (single-precision)"))
  ;[0.01013 0 0.15 0.5] LIFE AND DESTROY ENEMY
  (`KismetSystemLibrary.PrintText` (`KismetTextLibrary.Conv_DoubleToText` (`HealthComponent.GetHealth` (`self.m_healthComponent`)) "HalfToEven") false false (struct :`G` 0.66 :`B` 1.0 :`A` 1.0) 2.0 "VIDA ENEMIGO"))

(event `self.DamageCollision.OnComponentBeginOverlap`
  (params (OverlappedComponent :type "PrimitiveComponent Object Reference") (OtherActor :type "Actor Object Reference") (OtherComp :type "PrimitiveComponent Object Reference") (OtherBodyIndex :type Integer) (bFromSweep :type Boolean) (SweepResult :type "HitResult Structure (by ref)"))
  ;[0.15 8.3e-05 0.0334 0.5] Damag collision chaser enemy
)

(event `self.ReceiveBeginPlay`
  ;[0.03395 0 0.15 0.5] Begin Play
  (add `HealthComponent.OnHealthChanged` (`self.m_healthComponent`) (delegate `DamageFeedback`)))

(event `DamageFeedback`
  (params (Current :type "Float (single-precision)") (Max :type "Float (single-precision)") (Delta :type "Float (single-precision)") (InstigatorActor :type "Actor Object Reference"))
  ;[0.03395 0 0.15 0.5] Begin Play
  (bind (_direction _newtrack_0) (`Timeline|Timeline` :!via `PlayFromStart` :!label _label_3)
    (:`Update`
      (`MeshComponent.SetColorParameterValueOnMaterials` (`self.Mesh`) "Color" (`KismetMathLibrary.LinearColorLerp` (struct :`R` 1.0 :`G` 1.0 :`B` 1.0) (struct :`R` 1.0 :`A` 1.0) _newtrack_0))
      (`KismetSystemLibrary.Delay` 1.0)
      (goto _label_3 :!via `Stop`))))

(event `AttackFeedback`
  ;[0.003269 0.15 0.01005 0.5] Attack Feedback
  (bind (_direction _newtrack_0) (`Timeline|Timeline_0` :!via `PlayFromStart` :!label _label_4)
    (:`Update`
      (`MeshComponent.SetColorParameterValueOnMaterials` (`self.Mesh`) "Color" (`KismetMathLibrary.LinearColorLerp` (struct :`R` 1.0 :`G` 1.0 :`B` 1.0) (struct :`R` 1.0 :`G` 0.782079 :`A` 1.0) _newtrack_0))
      (`KismetSystemLibrary.Delay` 2.0)
      (goto _label_4 :!via `Stop`))))

(event `DashEnemy`
  ;[0.15 0.1213 0.01064 0.5] Dash Enemy
)

(fn `UserConstructionScript`)