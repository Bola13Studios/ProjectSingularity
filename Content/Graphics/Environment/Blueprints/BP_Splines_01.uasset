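; BP_Splines_01 is an environment tool that lays a chosen static mesh along an editable spline.
; Its construction script divides the spline by a segment length and adds a spline mesh component per step, with a configurable forward axis and query and physics collision.
; Each segment takes positions and tangents from the spline in local space, with tangents clamped to the segment length to limit distortion.
; The event graph has no active logic.
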(fn `UserConstructionScript`
  (bind _spline (`self.Spline`))
  (bind _spline_lenght (`self.Spline_Lenght`))
  (bind _spline_lenght_2 (`self.Spline_Lenght`))
  (for _index (range (+ (`KismetMathLibrary.FTrunc` (/ (`SplineComponent.GetSplineLength` (`self.Spline`)) _spline_lenght_2)) 1))
    (bind _returnvalue (`AddComponent|NODE_AddSplineMeshComponent-0`))
    (`StaticMeshComponent.SetStaticMesh` _returnvalue (`self.New_Mesh`))
    (`SplineMeshComponent.SetForwardAxis` _returnvalue (`self.In Forward Axis`) true)
    (`PrimitiveComponent.SetCollisionEnabled` _returnvalue "QueryAndPhysics")
    (bind _returnvalue_2 (* _index _spline_lenght_2))
    (bind _returnvalue_3 (* (+ _index 1) _spline_lenght_2))
    (`SplineMeshComponent.SetStartAndEnd` _returnvalue (`SplineComponent.GetLocationAtDistanceAlongSpline` _spline _returnvalue_2 "Local") (`KismetMathLibrary.ClampVectorSize` (`SplineComponent.GetTangentAtDistanceAlongSpline` _spline _returnvalue_2 "Local") 0.0 _spline_lenght) (`SplineComponent.GetLocationAtDistanceAlongSpline` _spline _returnvalue_3 "Local") (`KismetMathLibrary.ClampVectorSize` (`SplineComponent.GetTangentAtDistanceAlongSpline` _spline _returnvalue_3 "Local") 0.0 _spline_lenght) true)))